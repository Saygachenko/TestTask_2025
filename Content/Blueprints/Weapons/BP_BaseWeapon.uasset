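; BP_BaseWeapon is a weapon base whose start-fire, stop-fire and make-shot functions are empty stubs.
; On BeginPlay it caches its owning Pawn.
; CalculateTrace runs a debug-drawn line trace from the muzzle socket, ignoring the owner, and returns the hit.
; The trace end is the muzzle-to-viewpoint offset projected onto the view direction scaled by ShootDistance, without adding a world origin.
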(event `self.ReceiveBeginPlay`
  (bind _aspawn (cast `Pawn` (`self.GetOwner`)))
  (set `self.OwnerPawn` _aspawn))

(fn `CalculateTrace`
  (returns (ReturnValue :type Boolean) (OutHit :type "HitResult Structure"))
  (bind _returnvalue_location (`KismetMathLibrary.BreakTransform` (`SceneComponent.GetSocketTransform` (`self.SM_Weapon`) (`self.MuzzleSocketName`) "RTS_World")))
  (bind (_location _rotation) (`Controller.GetPlayerViewPoint` (`Pawn.GetController` (`self.OwnerPawn`))))
  (bind (_outhit _returnvalue) (`KismetSystemLibrary.LineTraceSingle` _returnvalue_location (`KismetMathLibrary.Vector_ProjectOnToNormal` (- _returnvalue_location _location) (* (`KismetMathLibrary.GetForwardVector` _rotation) (`self.ShootDistance`))) "TraceTypeQuery4" false (`|MakeArray` (`self.OwnerPawn`) :!type "Actor Object Reference") "ForOneFrame"))
  (return _returnvalue _outhit))

(fn `MakeShot`)

(fn `StartFireWeapon`)

(fn `StopFireWeapon`)

(fn `UserConstructionScript`)