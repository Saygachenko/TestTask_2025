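; Automatic rifle weapon Blueprint that overrides its parent's firing functions to shoot hitscan rounds.
; Starting fire shoots at once and repeats MakeShot on a looping FireRate timer until stopped or out of ammo.
; Each shot line-traces from the muzzle socket, using a random spread cone around the player's view direction, with debug drawing.
; Hits apply damage, play impact FX and consume ammo, while a missed trace stops firing.
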(fn `CalculateTrace`
  (returns (ReturnValue :type Boolean) (OutHit :type "HitResult Structure"))
  (bind _returnvalue_location (`KismetMathLibrary.BreakTransform` (`SceneComponent.GetSocketTransform` (`self.SM_Weapon`) (`self.MuzzleSocketName`) "RTS_World")))
  (bind (_location _rotation) (`Controller.GetPlayerViewPoint` (`Pawn.GetController` (`self.OwnerPawn`))))
  (`parent.CalculateTrace`)
  (bind (_outhit _returnvalue) (`KismetSystemLibrary.LineTraceSingle` :`Start` _returnvalue_location :`End` (`KismetMathLibrary.Vector_ProjectOnToNormal` (- _returnvalue_location _location) (* (`KismetMathLibrary.RandomUnitVectorInConeInDegrees` (`KismetMathLibrary.GetForwardVector` _rotation) (`self.BulletSpread`)) (`self.ShootDistance`))) :`TraceChannel` "TraceTypeQuery4" :`DrawDebugType` "ForOneFrame"))
  (return _returnvalue _outhit))

(fn `MakeDamage`
  (params (HitResult :type "HitResult Structure"))
  (`GameplayStatics.ApplyDamage` (`.HitActor` (`GameplayStatics.BreakHitResult` HitResult)) (`self.BaseDamage`) (`Pawn.GetController` (`self.OwnerPawn`)) self (`self.DamageType `)))

(fn `MakeShot`
  (`parent.MakeShot`)
  (bind _result (`self.IsAmmoEmpty`))
  (if _result
    (`self.StopFireWeapon`)
    (else
      (bind (_returnvalue _outhit) (`self.CalculateTrace`))
      (if _returnvalue
        (`self.MakeDamage` _outhit)
        (`/Game/Components/BP_WeaponFXComponent.PlayImpactFX` (`self.BP_WeaponFXComponent`) _outhit)
        (`self.DecreaseAmmo`)
        (else
          (`self.StopFireWeapon`))))))

(fn `StartFireWeapon`
  (`parent.StartFireWeapon`)
  (`KismetSystemLibrary.K2_SetTimer` null "MakeShot" (`self.FireRate`) true)
  (`self.MakeShot`))

(fn `StopFireWeapon`
  (`parent.StopFireWeapon`)
  (`KismetSystemLibrary.K2_ClearTimer` null "MakeShot"))

(fn `UserConstructionScript`
  (`parent.UserConstructionScript`))