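; Actor component on the third-person character that detects interactable actors the player camera is looking at.
; On BeginPlay it caches the character and starts a looping timer that runs a sphere trace forward from the camera manager.
; A newly hit actor implementing BP_InteractionInterface becomes LookAtActor and has its look-at message printed.
; LookAtActor clears only when the trace hits nothing.
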(event `self.ReceiveBeginPlay`
  (bind _asbp_third_person_character (cast `/Game/ThirdPerson/Blueprints/BP_ThirdPersonCharacter` (`self.GetOwner`)))
  (set `self.Character_Ref` _asbp_third_person_character)
  (`KismetSystemLibrary.K2_SetTimer` null "InteractionTrace" 0.1 true))

(fn `InteractionTrace`
  (bind _returnvalue (`GameplayStatics.GetPlayerCameraManager` 0))
  (bind _returnvalue_2 (`Actor.K2_GetActorLocation` _returnvalue))
  (bind (_outhit _returnvalue_3) (`KismetSystemLibrary.SphereTraceSingle` :`Start` _returnvalue_2 :`End` (+ _returnvalue_2 (* (`Actor.GetActorForwardVector` _returnvalue) (`self.LenghtTrace`))) :`Radius` (`self.SphereTraceRadios`) :`TraceChannel` "TraceTypeQuery3" :`DrawDebugType` "ForOneFrame"))
  (if _returnvalue_3
    (bind (_bblockinghit _binitialoverlap _time _distance _location _impactpoint _normal _impactnormal _physmat _hitactor) (`GameplayStatics.BreakHitResult` _outhit))
    (if (!= _hitactor (`self.LookAtActor`))
      (if (`KismetSystemLibrary.DoesImplementInterface` _hitactor "/Game/Interfaces/BP_InteractionInterface.BP_InteractionInterface_C")
        (bind _output_get (set `self.LookAtActor` _hitactor))
        (bind _message (message `/Game/Interfaces/BP_InteractionInterface.LookAt` _output_get))
        (`KismetSystemLibrary.PrintString` (`KismetTextLibrary.Conv_TextToString` _message))))
    (else
      (set `self.LookAtActor` null))))