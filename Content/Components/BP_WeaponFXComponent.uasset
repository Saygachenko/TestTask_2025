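; BP_WeaponFXComponent is a component that plays weapon impact effects at a hit location.
; PlayImpactFX looks up the hit's physical material in an impact data map, falling back to default data when none matches.
; It spawns the Niagara effect along the surface normal and a decal facing into the surface, which fades out and destroys itself using the data's timings.
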(fn `PlayImpactFX`
  (params (Hit :type "HitResult Structure"))
  (locals (Effect_Local :type "/Game/Structs/VFX/BP_ImpactData Structure"))
  (bind (_bblockinghit _binitialoverlap _time _distance _location _impactpoint _normal _impactnormal _physmat) (`GameplayStatics.BreakHitResult` Hit))
  (bind (_value _returnvalue) (`BlueprintMapLibrary.Map_Find` (`self.ImpactDataMap`) _physmat))
  (bind (_material _size _lifetime _fadeouttime) (break `/Game/Structs/VFX/BP_DecalData` (`.DecalData_5_E40B3B044BABFE64B1D410ABB125CED9` (break `/Game/Structs/VFX/BP_ImpactData` (`local.Effect_Local`)))))
  (set `local.Effect_Local` (`self.DefaultImpactData`))
  (if (`KismetSystemLibrary.IsValid` _physmat)
    (if _returnvalue
      (bind _output_get (set `local.Effect_Local` _value))))
  (`NiagaraFunctionLibrary.SpawnSystemAtLocation` (`.NiagaraEffect_4_AC1D01414A4587A0C7F016A6FA344194` (break `/Game/Structs/VFX/BP_ImpactData` _output_get)) _impactpoint (`KismetMathLibrary.Conv_VectorToRotator` _impactnormal))
  (bind _returnvalue_2 (`GameplayStatics.SpawnDecalAtLocation` _material _size _impactpoint (`KismetMathLibrary.Conv_VectorToRotator` (* _impactnormal -1.0))))
  (`DecalComponent.SetFadeOut` _returnvalue_2 _lifetime _fadeouttime true))