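; BP_Door is an interactable door actor that swings open and closed when the player interacts with it.
; Interactwith alternates through a FlipFlop between playing and reversing a timeline, whose float curve lerps the door component's relative yaw between 0 and 90 degrees.
; LookAt returns an "Interact:" prompt text built from the actor's display name.
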(event `/Game/TestTask_2025/Interfaces/BP_InteractionInterface.InteractWith`
  (params (Instigator :type "Actor Object Reference"))
  (`/Engine/EditorBlueprintResources/StandardMacros.FlipFlop`
    (:`A`
      (bind (_direction _doorfloat) (`Timeline|OpedTheDoorTimeLine` :!label _label)
        (:`Update`
          (`SceneComponent.K2_SetRelativeRotation` (`self.Door`) (`KismetMathLibrary.MakeRotator` 0.0 0.0 (`KismetMathLibrary.Lerp` 0.0 90.0 _doorfloat)) false false))))
    (:`B`
      (goto _label :!via `Reverse`))))

(fn `LookAt`
  (returns (Message :type Text))
  (return (`KismetTextLibrary.Conv_StringToText` (`KismetStringLibrary.Concat_StrStr` "Interact: " (`KismetSystemLibrary.GetDisplayName` self)))))

(fn `UserConstructionScript`
  (`parent.UserConstructionScript`))