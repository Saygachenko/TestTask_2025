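; Base weapon Blueprint providing ammo, tracing and muzzle effects, with empty start, stop and shot functions as override points.
; BeginPlay caches the owning pawn and copies default ammo; DecreaseAmmo stops fire and signals when a clip empties with ammo remaining.
; ChangeClip refills bullets, spending a clip unless infinite.
; CalculateTrace traces from the muzzle socket to an endpoint projected onto the scaled view direction, without adding an origin, ignoring the owner.
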(event `self.ReceiveBeginPlay`
  (bind _aspawn (cast `Pawn` (`self.GetOwner`)))
  (set `self.OwnerPawn` _aspawn)
  (set `self.CurrentAmmo` (`self.DefaultAmmo`)))

(fn `CalculateTrace`
  (returns (ReturnValue :type Boolean) (OutHit :type "HitResult Structure"))
  (bind _returnvalue_location (`KismetMathLibrary.BreakTransform` (`SceneComponent.GetSocketTransform` (`self.SM_Weapon`) (`self.MuzzleSocketName`) "RTS_World")))
  (bind (_location _rotation) (`Controller.GetPlayerViewPoint` (`Pawn.GetController` (`self.OwnerPawn`))))
  (bind (_outhit _returnvalue) (`KismetSystemLibrary.LineTraceSingle` _returnvalue_location (`KismetMathLibrary.Vector_ProjectOnToNormal` (- _returnvalue_location _location) (* (`KismetMathLibrary.GetForwardVector` _rotation) (`self.ShootDistance`))) "TraceTypeQuery4" false (`|MakeArray` (`self.OwnerPawn`) :!type "Actor Object Reference")))
  (return _returnvalue _outhit))

(fn `CanReload`
  (returns (Result :type Boolean))
  (bind ((`Bullets_6_1E539B6F4344442ABC9E128215E8E4CB` _bullets) (`Clips_7_0A5E0FDC4055EBA0CB4F298BFF1B4821` _clips)) (break `/Game/TestTask_2025/Structs/Weapons/BP_AmmoDataStruct` (`self.CurrentAmmo`)))
  (return (and (< _bullets (`.Bullets_6_1E539B6F4344442ABC9E128215E8E4CB` (break `/Game/TestTask_2025/Structs/Weapons/BP_AmmoDataStruct` (`self.DefaultAmmo`)))) (> _clips 0))))

(fn `ChangeClip`
  (bind ((`Clips_7_0A5E0FDC4055EBA0CB4F298BFF1B4821` _clips) (`Infinite_5_C523FEE245EF22CC70FEEAB1D9E5D8D8` _infinite)) (break `/Game/TestTask_2025/Structs/Weapons/BP_AmmoDataStruct` (`self.CurrentAmmo`)))
  (if (not (`.Infinite_5_C523FEE245EF22CC70FEEAB1D9E5D8D8` (break `/Game/TestTask_2025/Structs/Weapons/BP_AmmoDataStruct` (`self.CurrentAmmo`))))
    (if (== (`.Clips_7_0A5E0FDC4055EBA0CB4F298BFF1B4821` (break `/Game/TestTask_2025/Structs/Weapons/BP_AmmoDataStruct` (`self.CurrentAmmo`))) 0)
      (`KismetSystemLibrary.PrintString` "No more clips!")
      (else
        (`/Engine/EditorBlueprintResources/StandardMacros.DecrementInt` _clips
          (:`  `
            (set `self.CurrentAmmo` (make `/Game/TestTask_2025/Structs/Weapons/BP_AmmoDataStruct` (`.Bullets_6_1E539B6F4344442ABC9E128215E8E4CB` (break `/Game/TestTask_2025/Structs/Weapons/BP_AmmoDataStruct` (`self.DefaultAmmo`))) _clips _infinite) :!label _label)))))
    (else
      (goto _label))))

(fn `DecreaseAmmo`
  (if (== (`.Bullets_6_1E539B6F4344442ABC9E128215E8E4CB` (break `/Game/TestTask_2025/Structs/Weapons/BP_AmmoDataStruct` (`self.CurrentAmmo`))) 0)
    (`KismetSystemLibrary.PrintString` "Clip is empty!")
    (else
      (`/Engine/EditorBlueprintResources/StandardMacros.DecrementInt` (`.Bullets_6_1E539B6F4344442ABC9E128215E8E4CB` (break `/Game/TestTask_2025/Structs/Weapons/BP_AmmoDataStruct` (`self.CurrentAmmo`)))
        (:`  `
          (`self.LogAmmo`)
          (bind _result (`self.IsClipEmpty`))
          (bind _result_2 (`self.IsAmmoEmpty`))
          (if (and (not _result_2) _result)
            (`self.StopFireWeapon`)
            (`self.OnClipEmptySignature`)))))))

(fn `IsAmmoEmpty`
  (returns (Result :type Boolean))
  (bind ((`Clips_7_0A5E0FDC4055EBA0CB4F298BFF1B4821` _clips) (`Infinite_5_C523FEE245EF22CC70FEEAB1D9E5D8D8` _infinite)) (break `/Game/TestTask_2025/Structs/Weapons/BP_AmmoDataStruct` (`self.CurrentAmmo`)))
  (bind _result (`self.IsClipEmpty`))
  (return (and _result (== _clips 0) (not _infinite))))

(fn `IsClipEmpty`
  (returns (Result :type Boolean))
  (return (== (`.Bullets_6_1E539B6F4344442ABC9E128215E8E4CB` (break `/Game/TestTask_2025/Structs/Weapons/BP_AmmoDataStruct` (`self.CurrentAmmo`))) 0)))

(fn `LogAmmo`
  (bind (_bullets _clips _infinite) (break `/Game/TestTask_2025/Structs/Weapons/BP_AmmoDataStruct` (`self.CurrentAmmo`)))
  (`KismetSystemLibrary.PrintString` (`KismetStringLibrary.Concat_StrStr` "Ammo: " (`KismetStringLibrary.Conv_IntToString` _bullets) "   Infinite: " (`KismetStringLibrary.Conv_BoolToString` _infinite) "   Clips: " (`KismetStringLibrary.Conv_IntToString` _clips))))

(fn `MakeShot`)

(fn `SpawnMuzzleFX`
  (returns (Result :type "NiagaraComponent Object Reference"))
  (bind _returnvalue (`NiagaraFunctionLibrary.SpawnSystemAttached` (`self.MuzzleFX`) (`self.SM_Weapon`) (`self.MuzzleSocketName`) (0.0 0.0 0.0) (struct) "SnapToTarget" true))
  (return _returnvalue))

(fn `StartFireWeapon`)

(fn `StopFireWeapon`)

(fn `UserConstructionScript`)