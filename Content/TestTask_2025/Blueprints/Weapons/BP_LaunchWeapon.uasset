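; BP_LaunchWeapon is a weapon Blueprint that fires a spawned projectile, making one shot each time firing starts.
; MakeShot checks ammo, runs CalculateTrace, then spawns the projectile class at the muzzle socket, rotated toward the impact point or the trace end on a miss.
; Each shot sets the weapon as projectile owner, decreases ammo, and triggers muzzle FX and an attached fire sound.
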(fn `MakeShot`
  (bind _returnvalue (`SceneComponent.GetSocketLocation` (`self.SM_Weapon`) (`self.MuzzleSocketName`)))
  (`parent.MakeShot`)
  (bind _result (`self.IsAmmoEmpty`))
  (if (not _result)
    (bind (_returnvalue_2 _outhit) (`self.CalculateTrace`))
    (bind (_bblockinghit _binitialoverlap _time _distance _location _impactpoint _normal _impactnormal _physmat _hitactor _hitcomponent _hitbonename _bonename _hititem _elementindex _faceindex _tracestart _traceend) (`GameplayStatics.BreakHitResult` _outhit))
    (bind _returnvalue_3 (`|SpawnActorFromClass` (`self.ProjectileSpawnClass`) (`KismetMathLibrary.MakeTransform` _returnvalue (`KismetMathLibrary.FindLookAtRotation` _returnvalue (`KismetMathLibrary.SelectVector` _impactpoint _traceend _returnvalue_2))) "Undefined" "MultiplyWithRoot" null null))
    (`self.SetOwner` _returnvalue_3 self)
    (`self.DecreaseAmmo`)
    (`self.SpawnMuzzleFX`)
    (`GameplayStatics.SpawnSoundAttached` (`self.FireSound`) (`self.SM_Weapon`) (`self.MuzzleSocketName`) (0.0 0.0 0.0) (struct) "KeepRelativeOffset" false 1.0 1.0 0.0 null null)))

(fn `StartFireWeapon`
  (`parent.StartFireWeapon`)
  (`self.MakeShot`))

(fn `StopFireWeapon`
  (`parent.StopFireWeapon`))

(fn `UserConstructionScript`
  (`parent.UserConstructionScript`))