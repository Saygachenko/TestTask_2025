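; BP_Projectile is a weapon projectile that deals radial damage and destroys itself when its sphere collision hits something.
; BeginPlay sets its lifespan; on hit it stops moving, applies damage and plays impact FX through BPWeaponFXComponent.
; Helpers resolve the instigator pawn and controller through the owning BP_BaseWeapon's owner, so the shooter is ignored and credited.
; SetShotDirection is an empty stub, and Tick calls GetPawn without using the result.
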(event `self.ReceiveBeginPlay`
  (`self.SetLifeSpan` (`self.LifeSeconds`)))

(event `self.ReceiveTick`
  (params (DeltaSeconds :type "Float (single-precision)"))
  (`self.GetPawn`))

(event `self.SphereCollision.OnComponentHit`
  (params (HitComponent :type "PrimitiveComponent Object Reference") (OtherActor :type "Actor Object Reference") (OtherComp :type "PrimitiveComponent Object Reference") (NormalImpulse :type "Vector Structure") (Hit :type "HitResult Structure (by ref)"))
  (`MovementComponent.StopMovementImmediately` (`self.ProjectileMovement`))
  (bind _ownercontroller (`self.GetController`))
  (bind _ownerpawn (`self.GetPawn`))
  (`GameplayStatics.ApplyRadialDamage` (`self.BaseDamage`) (`self.K2_GetActorLocation`) (`self.BaseDamageRadius`) (`self.DamageTypeClass`) (`|MakeArray` _ownerpawn :!type "Actor Object Reference") self _ownercontroller (`self.DoFullDamage`))
  (`/Game/TestTask_2025/Components/BP_WeaponFXComponent.PlayImpactFX` (`self.BP_WeaponFXComponent`) Hit)
  (`self.K2_DestroyActor`))

(fn `GetController`
  (returns (OwnerController :type "Controller Object Reference"))
  (bind _asbp_base_weapon (cast `/Game/TestTask_2025/Blueprints/Weapons/BP_BaseWeapon` (`self.GetOwner`)))
  (return (`self.GetInstigatorController` (`self.GetOwner` _asbp_base_weapon))))

(fn `GetPawn`
  (returns (OwnerPawn :type "Pawn Object Reference"))
  (bind _asbp_base_weapon (cast `/Game/TestTask_2025/Blueprints/Weapons/BP_BaseWeapon` (`self.GetOwner`)))
  (return (`self.GetInstigator` (`self.GetOwner` _asbp_base_weapon))))

(fn `SetShotDirection`
  (params (Direction :type "Vector Structure")))

(fn `UserConstructionScript`)