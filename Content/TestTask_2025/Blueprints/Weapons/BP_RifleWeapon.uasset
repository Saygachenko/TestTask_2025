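; BP_RifleWeapon is an automatic hitscan rifle, firing immediately and then on a looping timer until stopped or out of ammo.
; Each shot line-traces from the muzzle along the controller's view direction with random cone spread, applies damage and impact FX on hit, and decreases ammo.
; Muzzle FX and looping-fire audio components are created once and toggled with firing, while each shot spawns a tracer given its end point.
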(fn `CalculateTrace`
  (returns (ReturnValue :type Boolean) (OutHit :type "HitResult Structure"))
  (bind _returnvalue_location (`KismetMathLibrary.BreakTransform` (`SceneComponent.GetSocketTransform` (`self.SM_Weapon`) (`self.MuzzleSocketName`) "RTS_World")))
  (bind (_outhit _returnvalue) (`KismetSystemLibrary.LineTraceSingle` _returnvalue_location (+ _returnvalue_location (* (`KismetMathLibrary.RandomUnitVectorInConeInDegrees` (`KismetMathLibrary.GetForwardVector` (`.Rotation` (`Controller.GetPlayerViewPoint` (`Pawn.GetController` (`self.OwnerPawn`))))) (`self.BulletSpread`)) (`self.ShootDistance`))) "TraceTypeQuery4"))
  (return _returnvalue _outhit))

(fn `InitFX`
  (`|ExecutionSequence`
    (:`then_0`
      (`self.MuzzleFXComponent`
        (:`then`
          _)
        (:`else`
          (bind _result (`self.SpawnMuzzleFX`))
          (set `self.MuzzleFXComponent` _result))))
    (:`then_1`
      (`self.FireAudioComponent`
        (:`then`
          _)
        (:`else`
          (bind _returnvalue (`GameplayStatics.SpawnSoundAttached` (`self.FireSound`) (`self.SM_Weapon`) (`self.MuzzleSocketName`) (0.0 0.0 0.0) (struct) "KeepRelativeOffset" false 1.0 1.0 0.0 null null))
          (set `self.FireAudioComponent` _returnvalue)))))
  (`self.SetFXActive` true))

(fn `MakeDamage`
  (params (HitResult :type "HitResult Structure"))
  (`GameplayStatics.ApplyDamage` (`.HitActor` (`GameplayStatics.BreakHitResult` HitResult)) (`self.BaseDamage`) (`Pawn.GetController` (`self.OwnerPawn`)) self (`self.DamageType `)))

(fn `MakeShot`
  (locals (TraceEnd_Local :type "Vector Structure" :default (0.0 0.0 0.0)))
  (bind _returnvalue_location (`KismetMathLibrary.BreakTransform` (`SceneComponent.GetSocketTransform` (`self.SM_Weapon`) (`self.MuzzleSocketName`) "RTS_World")))
  (`parent.MakeShot`)
  (bind _result (`self.IsAmmoEmpty`))
  (if _result
    (`self.StopFireWeapon`)
    (else
      (bind (_returnvalue _outhit) (`self.CalculateTrace`))
      (bind (_bblockinghit _binitialoverlap _time _distance _location _impactpoint _normal _impactnormal _physmat _hitactor _hitcomponent _hitbonename _bonename _hititem _elementindex _faceindex _tracestart _traceend) (`GameplayStatics.BreakHitResult` _outhit))
      (set `local.TraceEnd_Local` _traceend)
      (if _returnvalue
        (`self.MakeDamage` _outhit)
        (`/Game/TestTask_2025/Components/BP_WeaponFXComponent.PlayImpactFX` (`self.BP_WeaponFXComponent`) _outhit)
        (set `local.TraceEnd_Local` _impactpoint))
      (`self.SpawnTraceFX` _returnvalue_location (`local.TraceEnd_Local`))
      (`self.DecreaseAmmo`))))

(fn `SetFXActive`
  (params (IsActive :type Boolean))
  (`|ExecutionSequence`
    (:`then_0`
      (bind _muzzlefxcomponent (`self.MuzzleFXComponent`)
        (:`then`
          (`NiagaraComponent.SetPaused` _muzzlefxcomponent (not IsActive))
          (`SceneComponent.SetVisibility` _muzzlefxcomponent IsActive true))
        (:`else`)))
    (:`then_1`
      (bind _fireaudiocomponent (`self.FireAudioComponent`)
        (:`then`
          (if IsActive
            (`AudioComponent.Play` _fireaudiocomponent 0.0)
            (else
              (`AudioComponent.Stop` _fireaudiocomponent))))
        (:`else`)))))

(fn `SpawnTraceFX`
  (params (TraceStart :type "Vector Structure") (TraceEnd :type "Vector Structure"))
  (bind _returnvalue (`NiagaraFunctionLibrary.SpawnSystemAtLocation` (`self.TraceFX`) TraceStart))
  (`NiagaraComponent.SetVariableVec3` _returnvalue (`KismetStringLibrary.Conv_StringToName` (`self.TraceTargetName`)) TraceEnd))

(fn `StartFireWeapon`
  (`parent.StartFireWeapon`)
  (`self.InitFX`)
  (`KismetSystemLibrary.K2_SetTimer` null "MakeShot" (`self.FireRate`) true)
  (`self.MakeShot`))

(fn `StopFireWeapon`
  (`parent.StopFireWeapon`)
  (`KismetSystemLibrary.K2_ClearTimer` null "MakeShot")
  (`self.SetFXActive` false))

(fn `UserConstructionScript`
  (`parent.UserConstructionScript`))