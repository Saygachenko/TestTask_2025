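; Health component that tracks its owner's health and broadcasts health-change and death events.
; It binds to the owner's any-damage event, subtracts damage through a clamped setter and fires OnDeath at zero.
; If AutoHealth is on, non-lethal damage restarts a delayed looping timer that regenerates health until full.
; Each regeneration tick also broadcasts a second health change with a value of zero, after the setter's own broadcast.
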(event `self.ReceiveBeginPlay`
  (`self.SetHealth` (`self.MaxHealth`))
  (add `Actor.OnTakeAnyDamage` (`self.GetOwner`) (`|CreateDelegate` :!event `OnTakeAnyDamageEvent`)))

(event `OnTakeAnyDamageEvent`
  (params (DamagedActor :type "Actor Object Reference") (Damage :type "Float (single-precision)") (DamageType :type "DamageType Object Reference") (InstigatedBy :type "Controller Object Reference") (DamageCauser :type "Actor Object Reference"))
  (bind _newparam (`self.IsDead`))
  (if (not (or _newparam (<= Damage 0.0)))
    (`KismetSystemLibrary.K2_ClearTimer` null "HealthUpdate")
    (`self.SetHealth` (- (`self.Health`) Damage))
    (bind _newparam_2 (`self.IsDead`))
    (if _newparam_2
      (`self.FOnDeath`)
      (elif (`self.AutoHealth`)
        (`KismetSystemLibrary.K2_SetTimer` null "HealthUpdate" (`self.HelathUpdateTime`) true false (`self.HealthDelay`))))))

(fn `GetHealth`
  (returns (OutHealth :type "Float (double-precision)"))
  (return (`self.Health`)))

(fn `HealthUpdate`
  (`self.SetHealth` (+ (`self.Health`) (`self.HealthModifier`)))
  (`self.FOnHealthChange` 0.0)
  (if (`KismetMathLibrary.NearlyEqual_FloatFloat` (`self.Health`) (`self.MaxHealth`))
    (`KismetSystemLibrary.K2_ClearTimer` null "HealthUpdate")))

(fn `IsDead`
  (returns (NewParam :type Boolean))
  (return (`KismetMathLibrary.NearlyEqual_FloatFloat` (`self.Health`))))

(fn `SetHealth`
  (params (InHealth :type "Float (double-precision)"))
  (bind _output_get (set `self.Health` (`KismetMathLibrary.FClamp` InHealth 0.0 (`self.MaxHealth`))))
  (`self.FOnHealthChange` _output_get))